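; BP_BasePickup is a base pickup actor that can show its item name as an interact hint on the player's HUD.
; On BeginPlay it waits through a fixed delay, then caches IngameHud from the first player's BP_ShooterPlayerController.
; SetItemNameVisibility drives that HUD's interactable hint, passing Name to show it or empty text to hide it.
; GetInteractHitText returns empty text with the hint disabled.
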(event `self.ReceiveBeginPlay`
  (`KismetSystemLibrary.Delay` 3.0)
  (bind _asbp_shooter_player_controller (cast `/Game/Framework/BP_ShooterPlayerController` (`GameplayStatics.GetPlayerController` 0)))
  (set `self.Ingame Hud` (`/Game/Framework/BP_ShooterPlayerController.IngameHud` _asbp_shooter_player_controller)))

(event `/Game/Framework/Interfaces/BPI_Pickups.SetItemNameVisibility`
  (params (NewVisibility :type Boolean))
  (if NewVisibility
    (`/Game/Widgets/WBP_GameHud.SetInteractableHint` (`self.Ingame Hud`) true (`self.Name`))
    (else
      (`/Game/Widgets/WBP_GameHud.SetInteractableHint` (`self.Ingame Hud`) false ""))))

(fn `GetInteractHitText`
  (returns (InteractHitText :type Text) (ShowInteractHintText :type Boolean))
  (return "" false))

(fn `UserConstructionScript`)
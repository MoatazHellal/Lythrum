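; BP_Spectator is the spectator pawn that follows living BP_Hero_Lyth players in the shooter.
; On possession it shows the spectator menu, caches all heroes and calls Svr_AttachToPlayer to select the next one.
; That event cycles the index with wraparound, retrying after short delays past dead players, then snap-attaches and updates the displayed name.
; It also handles look pitch and pause toggling, and destroys itself when unpossessed.
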(event `InputAxis|LookUp`
  (params (AxisValue :type "Float (single-precision)"))
  (`self.AddControllerPitchInput` AxisValue))

(event `InputAction|PauseGame`
  (params (Key :type "Key Structure"))
  (:`Pressed`
    (bind _asbp_shooter_game_instance (cast `/Game/Framework/BP_ShooterGameInstance` (`GameplayStatics.GetGameInstance`)))
    (`/Game/Framework/BP_ShooterGameInstance.TogglePauseGame` _asbp_shooter_game_instance)))

(event `self.ReceivePossessed`
  (params (NewController :type "Controller Object Reference"))
  (bind _asbp_shooter_player_controller (cast `/Game/Framework/BP_ShooterPlayerController` NewController))
  (bind _output_get (set `self.As BP Shooter Player Controller` _asbp_shooter_player_controller))
  (`/Game/Framework/BP_ShooterPlayerController.ShowSpectatorMenu` _output_get)
  (bind _outactors (`GameplayStatics.GetAllActorsOfClass` "/Game/Characters/BP_Hero_Lyth.BP_Hero_Lyth_C"))
  (set `self.AllPlayers` _outactors)
  (`self.Svr_AttachToPlayer` true))

(event `Svr_AttachToPlayer`
  (params (IncreaseIndex :type Boolean))
  (bind _attachedplayer (`self.AttachedPlayer`))
  (bind _output (`|GetArrayItem` (`self.AllPlayers`) (`self.CurrentPlayerIndex`)))
  (bind _playerinfo_playername (break `/Game/SavedData/S_PlayerProfile` (`/Game/Framework/BP_ShooterGameInstance.PlayerInfo` (`/Game/Characters/BP_Hero_Lyth.As BP Shooter Game Instance` _attachedplayer))))
  (if IncreaseIndex
    (`/Engine/EditorBlueprintResources/StandardMacros.IncrementInt` (`self.CurrentPlayerIndex`) :!label _label
      (:`  `
        (if (== (`self.CurrentPlayerIndex`) (`KismetArrayLibrary.Array_Length` (`self.AllPlayers`)))
          (set `self.CurrentPlayerIndex` 0))
        (if (`/Game/Characters/BP_Hero_Lyth.IsAlive` _output)
          (set `self.AttachedPlayer` _output)
          (`self.K2_AttachToActor` _attachedplayer "None" "SnapToTarget" "SnapToTarget" "KeepRelative")
          (`/Game/Framework/BP_ShooterPlayerController.UpdateSpectedPlayerName` (`self.As BP Shooter Player Controller`) _playerinfo_playername)
          (elif (> (`KismetArrayLibrary.Array_Length` (`self.AllPlayers`)) 1)
            (`KismetSystemLibrary.Delay` 0.1)
            (goto _label)))))))

(event `self.ReceiveUnpossessed`
  (params (OldController :type "Controller Object Reference"))
  (`self.K2_DestroyActor`))

(fn `UserConstructionScript`)
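; BP_MenuPlayerController is the player controller for the multiplayer menu and lobby, using UI-only mouse input for the local player.
; InitialSetup loads or creates the saved player profile, then passes it through ServerUpdateLobby to BP_MenuGamemode to refresh the lobby.
; Other events show the lobby and loading-screen widgets, forward player names and level selection to the lobby widget, or destroy the session and open MainMenu.
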(event `CreateLoadingScreen`
  (`self.ShowLoadingScreenUI`))

(event `self.ReceiveBeginPlay`
  (if (`self.IsLocalController`)
    (set `self.bShowMouseCursor` true)
    (`WidgetBlueprintLibrary.SetInputMode_UIOnlyEx` self null)))

(event `EndClientSession`
  (`DestroySessionCallbackProxy.DestroySession` self
    (:`then`
      (`GameplayStatics.OpenLevel` "MainMenu"))))

(event `CreateLobbyMenu`
  (`self.ShowLobbyMenuUI`))

(event `InitialSetup`
  (`self.LoadSavedProfile`)
  (`self.ServerUpdateLobby` (`self.PlayerProfileInfo`)))

(event `ServerUpdateLobby`
  (params (PlayerProfile :type "/Game/SavedData/S_PlayerProfile Structure"))
  (set `self.PlayerProfileInfo` PlayerProfile)
  (bind _asbp_menu_gamemode (cast `/Game/Framework/BP_MenuGamemode` (`GameplayStatics.GetGameMode`)))
  (`/Game/Framework/BP_MenuGamemode.UpdateLobby` _asbp_menu_gamemode true true))

(event `UpdatePlayerNames`
  (params (PlayerProfiles :type "Array of /Game/SavedData/S_PlayerProfile Structure"))
  (bind _lobbywidget (`self.LobbyWidget`))
  (`/Engine/EditorBlueprintResources/StandardMacros.IsValid` _lobbywidget
    (:`Is Valid`
      (`/Game/Widgets/WBP_LobbyMenu.ClearPlayerNames` _lobbywidget)
      (`/Game/Widgets/WBP_LobbyMenu.UpdatePlayerNames` _lobbywidget PlayerProfiles))))

(event `UpdateLevelSelection`
  (params (LevelName :type Name))
  (bind _lobbywidget (`self.LobbyWidget`))
  (`/Engine/EditorBlueprintResources/StandardMacros.IsValid` _lobbywidget
    (:`Is Valid`
      (`/Game/Widgets/WBP_LobbyMenu.UpdateLevelSelection` _lobbywidget LevelName))))

(fn `LoadSavedProfile`
  (locals (LclSaveGameSlot :type String :default "PlayerProfile_Slot"))
  (bind _returnvalue (`GameplayStatics.DoesSaveGameExist` (`local.LclSaveGameSlot`)))
  (if (not _returnvalue)
    (bind _returnvalue_2 (`GameplayStatics.CreateSaveGameObject` "/Game/SavedData/BP_SaveGamePlayerProfile.BP_SaveGamePlayerProfile_C"))
    (`GameplayStatics.SaveGameToSlot` _returnvalue_2 (`local.LclSaveGameSlot`)))
  (bind _returnvalue_3 (`GameplayStatics.LoadGameFromSlot` (`local.LclSaveGameSlot`)))
  (bind _asbp_save_game_player_profile (cast `/Game/SavedData/BP_SaveGamePlayerProfile` _returnvalue_3))
  (set `self.PlayerProfileInfo` (`/Game/SavedData/BP_SaveGamePlayerProfile.PlayerProfile` _asbp_save_game_player_profile))
  (return))

(fn `ShowLoadingScreenUI`
  (`WidgetLayoutLibrary.RemoveAllWidgets`)
  (`/Engine/EditorBlueprintResources/StandardMacros.IsValid` (`self.LoadingScreenWidget`)
    (:`Is Valid`
      _)
    (:`Is Not Valid`
      (bind _returnvalue (`|CreateWidget` "/Game/Widgets/WBP_LoadingScreen.WBP_LoadingScreen_C" self))
      (set `self.LoadingScreenWidget` _returnvalue)))
  (`UserWidget.AddToViewport` (`self.LoadingScreenWidget`) 0)
  (return))

(fn `ShowLobbyMenuUI`
  (`/Engine/EditorBlueprintResources/StandardMacros.IsValid` (`self.LobbyWidget`)
    (:`Is Valid`
      _)
    (:`Is Not Valid`
      (bind _returnvalue (`|CreateWidget` "/Game/Widgets/WBP_LobbyMenu.WBP_LobbyMenu_C" self))
      (set `self.LobbyWidget` _returnvalue)))
  (`UserWidget.AddToViewport` (`self.LobbyWidget`) 0))

(fn `UserConstructionScript`)
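; BP_MenuGamemode is the menu game mode that manages players in the multiplayer lobby.
; When a player starts on the Lobby level, it stores their menu controller, creates the lobby menu and runs initial setup.
; UpdateLobby gathers profiles from connected controllers, copies them into shooter player states, and pushes names or the selected level name to each client.
; Logout removes the controller and refreshes the name list.
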(event `self.K2_OnLogout`
  (params (ExitingController :type "Controller Object Reference"))
  (bind _asbp_menu_player_controller (cast `/Game/Framework/BP_MenuPlayerController` ExitingController))
  (`KismetArrayLibrary.Array_RemoveItem` (`self.AllConnectedPlayers`) _asbp_menu_player_controller)
  (`self.UpdateLobby` true))

(event `self.HandleStartingNewPlayer`
  (params (NewPlayer :type "PlayerController Object Reference"))
  (bind _returnvalue (`GameplayStatics.GetCurrentLevelName` true))
  (switch `string` _returnvalue
    (:`Lobby`
      (bind _asbp_menu_player_controller (cast `/Game/Framework/BP_MenuPlayerController` NewPlayer))
      (`KismetArrayLibrary.Array_Add` (`self.AllConnectedPlayers`) _asbp_menu_player_controller)
      (`/Game/Framework/BP_MenuPlayerController.CreateLobbyMenu` _asbp_menu_player_controller)
      (`/Game/Framework/BP_MenuPlayerController.InitialSetup` _asbp_menu_player_controller))))

(event `UpdateLobby`
  (params (PlayerNames :type Boolean) (LevelName :type Boolean))
  (if PlayerNames
    (`KismetArrayLibrary.Array_Clear` (`self.AllPlayerProfiles`))
    (for _array_element (`self.AllConnectedPlayers`)
      (bind _playerprofileinfo (`/Game/Framework/BP_MenuPlayerController.PlayerProfileInfo` _array_element))
      (`KismetArrayLibrary.Array_Add` (`self.AllPlayerProfiles`) _playerprofileinfo)
      (bind _asbp_shooter_player_state (cast `/Game/Framework/BP_ShooterPlayerState` (`Controller.PlayerState` _array_element)))
      (set `/Game/Framework/BP_ShooterPlayerState.PlayerProfile` _playerprofileinfo _asbp_shooter_player_state)))
  (for _array_element_2 (`self.AllConnectedPlayers`)
    (if PlayerNames
      (`/Game/Framework/BP_MenuPlayerController.UpdatePlayerNames` _array_element_2 (`self.AllPlayerProfiles`)))
    (if LevelName
      (`/Game/Framework/BP_MenuPlayerController.UpdateLevelSelection` _array_element_2 (`self.SelectionLevelName`)))))

(fn `UserConstructionScript`)
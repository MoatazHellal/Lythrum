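; Player controller for a multiplayer shooter that manages each player's HUD, death, spectator and game-over screens, plus leaving the session.
; The local player gets the in-game HUD on BeginPlay, with events relaying countdown and interact hints to it.
; On death it shows the death screen only while some hero still lives.
; Spectating asks the game mode for a spectator, then Tick copies the watched player's aim yaw into control rotation.
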(event `self.ReceiveTick`
  (params (DeltaSeconds :type "Float (single-precision)"))
  (bind (_returnvalue_roll _returnvalue_pitch) (`KismetMathLibrary.BreakRotator` (`self.GetControlRotation`)))
  (if (`self.IsSpectating`)
    (bind _bp_spectator (`self.BP_Spectator`)
      (:`then`
        (bind (_aimrotation_roll _aimrotation_pitch _aimrotation_yaw) (`KismetMathLibrary.BreakRotator` (`/Game/Characters/BP_Hero_Lyth.AimRotation` (`/Game/Characters/BP_Spectator.AttachedPlayer` _bp_spectator))))
        (`self.SetControlRotation` (`KismetMathLibrary.MakeRotator` _returnvalue_roll _returnvalue_pitch _aimrotation_yaw)))
      (:`else`))))

(event `self.ReceiveBeginPlay`
  (if (`self.IsLocalPlayerController`)
    (`WidgetLayoutLibrary.RemoveAllWidgets`)
    (`self.ShowIngameHud`)
    (`/Game/Widgets/WBP_GameHud.UpdateHealth` (`self.IngameHud`) 100.0 false)
    (`WidgetBlueprintLibrary.SetInputMode_GameOnly` self)
    (set `self.bShowMouseCursor` false)))

(event `EnableAllInput`
  (`self.EnableInput` (`self.K2_GetPawn`) self))

(event `GameStartCountdown`
  (`/Game/Widgets/WBP_GameHud.StartGameCountdown` (`self.IngameHud`)))

(event `UnhideGameHud`
  (`Widget.SetVisibility` (`self.IngameHud`) "Visible"))

(event `EndClientSession`
  (bind _asbp_shooter_game_instance (cast `/Game/Framework/BP_ShooterGameInstance` (`GameplayStatics.GetGameInstance`)))
  (set `/Game/Framework/BP_ShooterGameInstance.MP_IsPauseMenuVisible` false _asbp_shooter_game_instance)
  (`DestroySessionCallbackProxy.DestroySession` self
    (:`then`
      (`GameplayStatics.OpenLevel` "MainMenu"))))

(event `Spectate`
  (set `self.IsSpectating` true)
  (bind _asbp_shooter_gamemode (cast `/Game/Framework/BP_Shooter_Gamemode` (`GameplayStatics.GetGameMode`)))
  (`/Game/Framework/BP_Shooter_Gamemode.SpawnSpectator` _asbp_shooter_gamemode self))

(event `ShowSpectatorMenu`
  (`/Game/Widgets/WBP_DeathScreen.ShowSpectatorMenu` (`self.DeathScreenWidget`) true)
  (set `self.bShowMouseCursor` false)
  (`WidgetBlueprintLibrary.SetInputMode_GameOnly` self))

(event `UpdateSpectedPlayerName`
  (params (PlayerName :type Text))
  (`/Game/Widgets/WBP_DeathScreen.UpdateSpectatedPlayerName` (`self.DeathScreenWidget`) PlayerName))

(event `ShowGameOverScreen`
  (`WidgetLayoutLibrary.RemoveAllWidgets`)
  (bind _returnvalue (`|CreateWidget` "/Game/Widgets/WBP_GameOver.WBP_GameOver_C" self))
  (`UserWidget.AddToViewport` _returnvalue 0))

(event `Hud_SetInteractHint`
  (params (NewVisibility :type Boolean) (HintText :type Text))
  (`/Game/Widgets/WBP_GameHud.SetInteractableHint` (`self.IngameHud`) NewVisibility HintText))

(fn `ShowDeathMenu`
  (locals (LclDeadPlayers :type Integer))
  (bind _ingamehud (`self.IngameHud`))
  (bind _ingamehud_2 (`self.IngameHud`))
  (bind _outactors (`GameplayStatics.GetAllActorsOfClass` "/Game/Characters/BP_Hero_Lyth.BP_Hero_Lyth_C"))
  (for _array_element _outactors
    (if (not (`/Game/Characters/BP_Hero_Lyth.IsAlive` _array_element))
      (`/Engine/EditorBlueprintResources/StandardMacros.IncrementInt` (`local.LclDeadPlayers`))))
  (if (== (`KismetArrayLibrary.Array_Length` _outactors) (`local.LclDeadPlayers`))
    (`/Engine/EditorBlueprintResources/StandardMacros.IsValid` _ingamehud_2
      (:`Is Valid`
        (`Widget.RemoveFromParent` _ingamehud_2)))
    (else
      (`/Engine/EditorBlueprintResources/StandardMacros.IsValid` _ingamehud
        (:`Is Valid`
          (`Widget.RemoveFromParent` _ingamehud)
          (`/Engine/EditorBlueprintResources/StandardMacros.IsValid` (`self.DeathScreenWidget`)
            (:`Is Valid`
              _)
            (:`Is Not Valid`
              (bind _returnvalue (`|CreateWidget` "/Game/Widgets/WBP_DeathScreen.WBP_DeathScreen_C" self))
              (set `self.DeathScreenWidget` _returnvalue)))
          (`UserWidget.AddToViewport` (`self.DeathScreenWidget`) 0)
          (`WidgetBlueprintLibrary.SetInputMode_UIOnlyEx` self null)
          (set `self.bShowMouseCursor` true)))))
  (return))

(fn `ShowIngameHud`
  (`/Engine/EditorBlueprintResources/StandardMacros.IsValid` (`self.IngameHud`)
    (:`Is Valid`
      _)
    (:`Is Not Valid`
      (bind _returnvalue (`|CreateWidget` "/Game/Widgets/WBP_GameHud.WBP_GameHud_C" self))
      (set `self.IngameHud` _returnvalue)))
  (`UserWidget.AddToViewport` (`self.IngameHud`) 0)
  (return))

(fn `UserConstructionScript`)
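; Shooter game mode that manages player spawning, match start and game over for solo and multiplayer games.
; It tracks connected controllers, takes the expected count from the game instance and restarts players at index-tagged PlayerStarts.
; LvlStart triggers each controller's countdown, then enables input.
; It can swap players to spectator pawns, and GMPlayedDied counts dead heroes and spectators, server-traveling to MainMenu when everyone is out.
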(event `self.K2_OnLogout`
  (params (ExitingController :type "Controller Object Reference"))
  (bind _asbp_shooter_player_controller (cast `/Game/Framework/BP_ShooterPlayerController` ExitingController))
  (`KismetArrayLibrary.Array_RemoveItem` (`self.AllConnectedPlayers`) _asbp_shooter_player_controller)
  (`/Engine/EditorBlueprintResources/StandardMacros.DecrementInt` (`self.NumExpectedPlayers`)))

(event `self.HandleStartingNewPlayer`
  (params (NewPlayer :type "PlayerController Object Reference"))
  (bind _asbp_shooter_player_controller (cast `/Game/Framework/BP_ShooterPlayerController` NewPlayer))
  (`KismetArrayLibrary.Array_Add` (`self.AllConnectedPlayers`) _asbp_shooter_player_controller)
  (bind _asbp_shooter_game_instance (cast `/Game/Framework/BP_ShooterGameInstance` (`GameplayStatics.GetGameInstance`)))
  (set `self.NumExpectedPlayers` (`/Game/Framework/BP_ShooterGameInstance.NumConnectedPlayers` _asbp_shooter_game_instance))
  (if (`/Game/Framework/BP_ShooterGameInstance.IsSoloGame` _asbp_shooter_game_instance)
    (set `self.NumExpectedPlayers` 1)
    (`self.RestartPlayerAtPlayerStart` (`|GetArrayItem` (`self.AllConnectedPlayers`)) (`self.K2_FindPlayerStart` null "0"))
    (`self.LvlStart`)
    (else
      (if (== (`self.NumExpectedPlayers`) (`KismetArrayLibrary.Array_Length` (`self.AllConnectedPlayers`)))
        (`KismetSystemLibrary.Delay` 0.5)
        (else
          (`KismetSystemLibrary.PrintString` "PIE Launch Enabled")))
      (for (_array_element _array_index) (`self.AllConnectedPlayers`)
        (`self.RestartPlayerAtPlayerStart` _array_element (`self.K2_FindPlayerStart` _array_element (`KismetStringLibrary.Conv_IntToString` _array_index))))
      (`self.LvlStart`))))

(event `LvlStart`
  (`KismetSystemLibrary.Delay` 0.2)
  (for _array_element (`self.AllConnectedPlayers`)
    (`/Game/Framework/BP_ShooterPlayerController.GameStartCountdown` _array_element))
  (`KismetSystemLibrary.Delay` 3.0)
  (for _array_element_2 (`self.AllConnectedPlayers`)
    (`/Game/Framework/BP_ShooterPlayerController.EnableAllInput` _array_element_2)))

(event `SpawnSpectator`
  (params (PlayerController :type "/Game/Framework/BP_ShooterPlayerController Object Reference"))
  (`Controller.UnPossess` PlayerController)
  (bind _returnvalue (`|SpawnActorFromClass` "/Game/Characters/BP_Spectator.BP_Spectator_C" (`KismetMathLibrary.MakeTransform` (0.0 0.0 0.0)) "Undefined" "OverrideRootScale" null null))
  (`Controller.Possess` PlayerController _returnvalue))

(event `GameOver`
  (for _array_element (`self.AllConnectedPlayers`)
    (`/Game/Framework/BP_ShooterPlayerController.ShowGameOverScreen` _array_element))
  (`KismetSystemLibrary.Delay` 3.0)
  (`KismetSystemLibrary.ExecuteConsoleCommand` "servertravel MainMenu" (`GameplayStatics.GetPlayerController` 0)))

(fn `GM_PlayedDied`
  (locals (LclDeadPlayers :type Integer))
  (for _array_element (`self.AllConnectedPlayers`)
    (bind _returnvalue (`Controller.K2_GetPawn` _array_element))
    (bind _asbp_hero_lyth (cast `/Game/Characters/BP_Hero_Lyth` _returnvalue)
      (:`then`
        (if (not (`/Game/Characters/BP_Hero_Lyth.IsAlive` _asbp_hero_lyth))
          (`/Engine/EditorBlueprintResources/StandardMacros.IncrementInt` (`local.LclDeadPlayers`) :!label _label)))
      (:`CastFailed`
        (cast `/Game/Characters/BP_Spectator` _returnvalue)
        (goto _label))))
  (if (== (`KismetArrayLibrary.Array_Length` (`self.AllConnectedPlayers`)) (`local.LclDeadPlayers`))
    (`self.GameOver`))
  (return))

(fn `UserConstructionScript`)